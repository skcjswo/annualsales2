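; Enemy actor that the player destroys by holding the interact input while inside its Sphere trigger.
; Sphere overlap with bp_character enables input, shows an Energybar widget and opens a gate, and leaving reverses this.
; Pressing starts a retriggerable delay that destroys the actor if interact is still held when it ends.
; A parallel timer, polled recursively, feeds hold progress to the widget, resetting it on release.
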(event `InputAction|interact`
  (params (Key :type "Key Structure"))
  (:`Pressed`
    (set `self.isHeld?` true)
    (`/Engine/EditorBlueprintResources/StandardMacros.Gate` true :!label _label
      (:`Exit`
        (`|ExecutionSequence`
          (:`then_0`
            (`KismetSystemLibrary.RetriggerableDelay` (`self.MaxHoldTime`))
            (if (`self.isHeld?`)
              (`self.K2_DestroyActor`)))
          (:`then_1`
            (`self.TImer1`)
            (`self.Update TImer1`))))))
  (:`Released`
    (set `self.isHeld?` false)))

(event `self.Sphere.OnComponentBeginOverlap`
  (params (OverlappedComponent :type "PrimitiveComponent Object Reference") (OtherActor :type "Actor Object Reference") (OtherComp :type "PrimitiveComponent Object Reference") (OtherBodyIndex :type Integer) (bFromSweep :type Boolean) (SweepResult :type "HitResult Structure (by ref)"))
  (cast `/Game/smson/bp/bp_character` OtherActor)
  (`self.EnableInput` (`GameplayStatics.GetPlayerController` 0))
  (bind _returnvalue (`|CreateWidget` "/Game/smson/bp/energybar.energybar_C"))
  (bind _output_get (set `self.widget ref` _returnvalue))
  (`UserWidget.AddToViewport` _output_get 0)
  (set `/Game/smson/bp/energybar.Max timeheld` (`self.MaxHoldTime`) _output_get)
  (goto _label :!via `Open`))

(event `Stop Timer1`
  (`KismetSystemLibrary.K2_PauseTimerHandle` (stale `TImer1` _returnvalue)))

(event `TImer1`
  (bind _returnvalue (`KismetSystemLibrary.K2_SetTimerDelegate` (delegate `TImer1`) (`self.MaxHoldTime`))))

(event `self.Sphere.OnComponentEndOverlap`
  (params (OverlappedComponent :type "PrimitiveComponent Object Reference") (OtherActor :type "Actor Object Reference") (OtherComp :type "PrimitiveComponent Object Reference") (OtherBodyIndex :type Integer))
  (cast `/Game/smson/bp/bp_character` OtherActor)
  (`self.DisableInput` (`GameplayStatics.GetPlayerController` 0))
  (`Widget.RemoveFromParent` (stale `self.Sphere.OnComponentBeginOverlap` _returnvalue))
  (goto _label :!via `Close`))

(event `Update TImer1`
  (bind _widget_ref (`self.widget ref`))
  (if (`self.isHeld?`)
    (set `/Game/smson/bp/energybar.Timeheld` (`KismetSystemLibrary.K2_GetTimerElapsedTimeHandle` (stale `TImer1` _returnvalue)) _widget_ref)
    (`KismetSystemLibrary.Delay` 0.1)
    (`self.Update TImer1`)
    (else
      (`self.Stop Timer1`)
      (set `/Game/smson/bp/energybar.Timeheld` 0.0 _widget_ref))))

(fn `UserConstructionScript`)