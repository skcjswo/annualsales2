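; Player character Blueprint for a three-lane runner that moves forward automatically.
; Tick feeds movement input along the control rotation's yaw, while A and D call ChangeLane to shift the clamped lane index left or right.
; A timeline lerps the actor's world Y to that lane's entry in LinePositions without sweeping, updating the current lane index as it plays.
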(event `self.ReceiveTick`
  (params (DeltaSeconds :type "Float (single-precision)"))
  ;[1 0.6698 0.8463] 달리기
  (`self.AddMovementInput` (`KismetMathLibrary.GetForwardVector` (`KismetMathLibrary.MakeRotator` 0.0 0.0 (.yaw (`self.GetControlRotation`))))))

(event `ChangeLane`
  (params (ShiftLane :type Integer))
  ;[0.8682 1 0.6323] 좌우 이동
  (set `self.TargetLaneIndex` (`KismetMathLibrary.Clamp` (+ ShiftLane (`self.CurrentLaneIndex`)) 0 2))
  (set `self.CurrentYPosition` (.y (`self.K2_GetActorLocation`)))
  (bind (_direction `_새_트랙_0`) (`Timeline|ChangeLaneTimeline` :!via `PlayFromStart`)
    (:`Update`
      (`self.K2_SetActorLocation` (`KismetMathLibrary.MakeVector` (.x (`self.K2_GetActorLocation`)) (`KismetMathLibrary.Lerp` (`self.CurrentYPosition`) (`|GetArrayItem` (`self.LinePositions`) (`self.TargetLaneIndex`)) `_새_트랙_0`) (.z (`self.K2_GetActorLocation`))))
      (set `self.CurrentLaneIndex` (`self.TargetLaneIndex`)))))

(event `Key|A`
  (params (Key :type "Key Structure"))
  ;[0.8682 1 0.6323] 좌우 이동
  (:`Pressed`
    (`self.ChangeLane` -1)))

(event `Key|D`
  (params (Key :type "Key Structure"))
  ;[0.8682 1 0.6323] 좌우 이동
  (:`Pressed`
    (`self.ChangeLane` 1)))

(fn `UserConstructionScript`)